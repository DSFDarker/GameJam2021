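; Hunter AI character that patrols on BeginPlay, either along a fixed path or at random, chosen by BPatrolPath.
; The construction script places four patrol markers and a box from variables; path mode caches the markers' world locations and loops through them, halting if a move fails.
; Random mode repeatedly moves to points within the box's extent, centred on world origin rather than the box, retrying on failure.
; Collected is a stub returning fixed values.
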(event EventBeginPlay
  (bind _target_point (Variables|Default|GetTarget_Point))
  (if (Variables|Patrol|GetB_Patrol_Path)
    (CallFunction|PatrolArraySetup)
    (AI|AIMoveTo self (Utilities|Array|Get(acopy) _target_point (Variables|Default|GetTarget_Ref)) 0 5.0 false :!label _label
      (:OnSuccess
        (bind _output_get (Variables|Default|SetTarget_Ref (+ (Variables|Default|GetTarget_Ref) 1)))
        (if (>= _output_get (Utilities|Array|Length _target_point))
          (Variables|Default|SetTarget_Ref 0)
          (goto _label)
          (else
            (goto _label)))))
    (else
      (AI|AIMoveTo self (Math|Random|RandomPointinBoundingBox "0, 0, 0" (Components|Box|GetScaledBoxExtent (Variables|Default|GetPatrol_Box))) 0 5.0 false :!label _label_2
        (:OnSuccess
          (goto _label_2))
        (:OnFail
          (goto _label_2))))))

(fn ConstructionScript
  (Transformation|SetRelativeLocation (Variables|Default|GetPatrol_01) (Math|Vector|MakeVector (Variables|Patrol|GetPatrol_01_X) (Variables|Patrol|GetPatrol_01_Y) 115.0) false false)
  (Transformation|SetRelativeLocation (Variables|Default|GetPatrol_02) (Math|Vector|MakeVector (Variables|Patrol|GetPatrol_02_X) (Variables|Patrol|GetPatrol_02_Y) 115.0) false false)
  (Transformation|SetRelativeLocation (Variables|Default|GetPatrol_03) (Math|Vector|MakeVector (Variables|Patrol|GetPatrol_03_X) (Variables|Patrol|GetPatrol_03_Y) 115.0) false false)
  (Transformation|SetRelativeLocation (Variables|Default|GetPatrol_04) (Math|Vector|MakeVector (Variables|Patrol|GetPatrol_04_X) (Variables|Patrol|GetPatrol_04_Y) 115.0) false false)
  (Transformation|SetWorldLocation (Variables|Default|GetPatrol_Box) (Math|Vector|MakeVector (Variables|Patrol|GetPatrol_Box_X) (Variables|Patrol|GetPatrol_Box_Y) 0.0) false false)
  (Components|Box|SetBoxExtent (Variables|Default|GetPatrol_Box) (Math|Vector|MakeVector (Variables|Patrol|GetPatrol_Box_X_Scale) (Variables|Patrol|GetPatrol_Box_Y_Scale) 6e+01) true))

(fn PatrolArraySetup
  (Variables|Default|SetTarget_Point (Utilities|Array|MakeArray (Transformation|GetWorldLocation (Variables|Default|GetPatrol_01)) (Transformation|GetWorldLocation (Variables|Default|GetPatrol_02)) (Transformation|GetWorldLocation (Variables|Default|GetPatrol_03)) (Transformation|GetWorldLocation (Variables|Default|GetPatrol_04)))))

(fn Collected
  (params (Input :type Boolean))
  (return false 1))