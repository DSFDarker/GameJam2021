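; BP_Player_Character is a player pawn that moves along its forward axis and turns by controller yaw from two input axes.
; The forward axis value is also stored as CharacterSpeed, and turning scales by a Speed variable and frame delta time.
; A BallotCheck function reports the Ballots count, and Collected prints a debug message and notifies the game mode, with both returning Success as false.
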(event Input|AxisEvents|InputAxisMoveUp
  (params (AxisValue :type Float%20%28single-precision%29))
  ;[1 1 1] Player Movement
  (Variables|Default|SetcharacterSpeed AxisValue)
  (Pawn|Input|AddMovementInput (Transformation|GetActorForwardVector) AxisValue false))

(event Input|AxisEvents|InputAxisMoveLeft
  (params (AxisValue :type Float%20%28single-precision%29))
  ;[1 1 1] Player Movement
  (Pawn|Input|AddControllerYawInput (* AxisValue (Utilities|Time|GetWorldDeltaSeconds) (Variables|Default|Getspeed))))

(fn ConstructionScript)

(fn BallotCheck
  (params (input :type Boolean))
  (return false (Variables|Default|Getballots)))

(fn Collected
  (params (Input :type Boolean))
  ;[1 1 1] Count Points
  (Development|PrintString "Player got message")
  (Class|BPIPlayer|Collected(Message) (Game|GetGameMode) false)
  (return false 0))