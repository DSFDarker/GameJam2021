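; Game mode for a ballot hunt game that keeps running Trump and Biden ballot totals and shows them on a HUD widget.
; BeginPlay creates the HUD and starts a looping timer that raises both totals by small random amounts, with Biden's range higher.
; Collected adds a random bonus to Trump's total, updates the HUD and returns the truncated count.
; BallotCheck is a stub that always reports failure with zero ballots.
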(event Custom|Ballot_Bumping
  (bind _hud (Variables|Default|GetHUD))
  (Variables|Default|SetTrump_BallotsCount (+ (Variables|Default|GetTrump_BallotsCount) (Math|Random|RandomFloatinRange 0.01 0.04)))
  (Variables|Default|SetBiden_BallotsCount (+ (Variables|Default|GetBiden_BallotsCount) (Math|Random|RandomFloatinRange 0.03 0.06)))
  (Variables|/Game/Blueprints/HUD.HUD_C|SetBallots _hud (Variables|Default|GetTrump_BallotsCount))
  (Variables|/Game/Blueprints/HUD.HUD_C|SetBiden_Ballot_Count _hud (Variables|Default|GetBiden_BallotsCount)))

(event EventBeginPlay
  ;[1 1 1] Add HUD
  (bind _returnvalue (UserInterface|CreateWidget "/Game/Blueprints/HUD.HUD_C"))
  (bind _output_get (Variables|Default|SetHUD _returnvalue))
  (UserInterface|Viewport|AddtoViewport _output_get 0)
  (Utilities|Time|SetTimerbyEvent (delegate Custom|Ballot_Bumping) 2.0 true))

(fn ConstructionScript)

(fn BallotCheck
  (params (input :type Boolean))
  (return false 0))

(fn Collected
  (params (Input :type Boolean))
  ;[1 1 1] Count Points
  (bind _output_get (Variables|Default|SetTrump_BallotsCount (+ (Variables|Default|GetTrump_BallotsCount) (Math|Random|RandomFloatinRange 0.03 0.07))))
  (bind _output_get_2 (Variables|/Game/Blueprints/HUD.HUD_C|SetBallots (Variables|Default|GetHUD) _output_get))
  (return true (Math|Float|Truncate _output_get_2)))