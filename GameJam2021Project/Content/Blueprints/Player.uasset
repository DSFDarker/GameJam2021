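; Player Blueprint that moves a physics-driven cube from movement input.
; Four input axis events scale their value by Speed and apply it as an impulse to PlayerCube, with Up and Down on world X and Left and Right on world Y.
; Direction sign comes from the axis values, and the impulses respect mass and are not scaled by delta time.
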(event Input|AxisEvents|InputAxisMoveUp
  (params (AxisValue :type Float%20%28single-precision%29))
  ;[1 1 1] Player Movement
  (Physics|AddImpulse (Variables|Default|GetPlayerCube) (Math|Vector|MakeVector (* AxisValue (Variables|Default|Getspeed)) 0.0 0.0) "None" false))

(event Input|AxisEvents|InputAxisMoveLeft
  (params (AxisValue :type Float%20%28single-precision%29))
  ;[1 1 1] Player Movement
  (Physics|AddImpulse (Variables|Default|GetPlayerCube) (Math|Vector|MakeVector 0.0 (* AxisValue (Variables|Default|Getspeed)) 0.0) "None" false))

(event Input|AxisEvents|InputAxisMoveDown
  (params (AxisValue :type Float%20%28single-precision%29))
  ;[1 1 1] Player Movement
  (Physics|AddImpulse (Variables|Default|GetPlayerCube) (Math|Vector|MakeVector (* AxisValue (Variables|Default|Getspeed)) 0.0 0.0) "None" false))

(event Input|AxisEvents|InputAxisMoveRight
  (params (AxisValue :type Float%20%28single-precision%29))
  ;[1 1 1] Player Movement
  (Physics|AddImpulse (Variables|Default|GetPlayerCube) (Math|Vector|MakeVector 0.0 (* AxisValue (Variables|Default|Getspeed)) 0.0) "None" false))

(fn ConstructionScript)